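; Base replicated projectile for spaceship weapons, with a configurable plasma trail colour, speed, damage and impact effect.
; ProjectileMovement takes its initial speed from Speed, and BeginPlay attaches the actor to SpaceshipRef when valid.
; On overlap with anything but its instigator, the server spawns impact FX through an event, applies damage credited to player pawn 0, then destroys itself.
; PlasmaColor's OnRep reapplies the trail's colour and template.
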(event `self.ReceiveBeginPlay`
  (bind _spaceshipref (`self.SpaceshipRef`)
    (:`then`
      (`self.K2_AttachToActor` _spaceshipref "None" "KeepWorld" "KeepWorld" "KeepWorld"))
    (:`else`
      _))
  (`/Engine/EditorBlueprintResources/ActorMacros.Switch Has Authority`
    (:`Authority`
      (set `self.PlasmaColor` (`self.PlasmaColor`)))))

(event `self.ReceiveTick`
  (params (DeltaSeconds :type "Float (single-precision)")))

(event `self.ProjectileColl.OnComponentBeginOverlap`
  (params (OverlappedComponent :type "PrimitiveComponent Object Reference") (OtherActor :type "Actor Object Reference") (OtherComp :type "PrimitiveComponent Object Reference") (OtherBodyIndex :type Integer) (bFromSweep :type Boolean) (SweepResult :type "HitResult Structure (by ref)"))
  (`/Engine/EditorBlueprintResources/ActorMacros.Switch Has Authority`
    (:`Authority`
      (if (!= OtherActor (`self.Instigator`))
        (`self.Rep Spawn Impact FX` (`self.Impact FX`) SweepResult)
        (`GameplayStatics.ApplyDamage` (`.HitActor` (`GameplayStatics.BreakHitResult` SweepResult)) (`self.Damage`) null (`GameplayStatics.GetPlayerPawn` 0))
        (`self.K2_DestroyActor`)))))

(event `Spawn Impact FX On Server`
  (params (ImpactFX :type "ParticleSystem Object Reference") (Hit :type "HitResult Structure (by ref)"))
  (`self.Rep Spawn Impact FX` ImpactFX Hit))

(event `Rep Spawn Impact FX`
  (params (ImpactFX :type "ParticleSystem Object Reference") (Hit :type "HitResult Structure (by ref)"))
  (bind (_bblockinghit _binitialoverlap _time _distance _location _impactpoint _normal _impactnormal _physmat _hitactor _hitcomponent _hitbonename) (`GameplayStatics.BreakHitResult` Hit))
  (`GameplayStatics.SpawnEmitterAttached` ImpactFX _hitcomponent _hitbonename _impactpoint (`KismetMathLibrary.Conv_VectorToRotator` _impactnormal) (`self.GetActorScale3D`) "KeepWorldPosition"))

(fn `GetIsPlayerOrEnemy`
  (params (`Other Comp` :type "PrimitiveComponent Object Reference"))
  (returns (IsPlayer :type Boolean) (IsOneOfThem :type Boolean))
  (bind _returnvalue (`|EnumInequality` (`PrimitiveComponent.GetCollisionResponseToChannel` `Other Comp` "ECC_GameTraceChannel2") "ECR_Ignore"))
  (return _returnvalue (or _returnvalue (`|EnumInequality` (`PrimitiveComponent.GetCollisionResponseToChannel` `Other Comp` "ECC_GameTraceChannel3") "ECR_Ignore"))))

(fn `OnRep_PlasmaColor`
  (bind _projectilefx (`self.ProjectileFX`))
  (`FXSystemComponent.SetColorParameter` _projectilefx "Plasma Color" (`self.PlasmaColor`))
  (`ParticleSystemComponent.SetTemplate` _projectilefx (`self.Trace FX`)))

(fn `UserConstructionScript`
  (bind _projectilefx (`self.ProjectileFX`))
  (`FXSystemComponent.SetColorParameter` _projectilefx "Plasma Color" (`self.PlasmaColor`))
  (`ParticleSystemComponent.SetTemplate` _projectilefx (`self.Trace FX`))
  (set `ProjectileMovementComponent.InitialSpeed` (`self.Speed`) (`self.ProjectileMovement`)))