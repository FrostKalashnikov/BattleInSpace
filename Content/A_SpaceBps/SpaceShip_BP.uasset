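; Spaceship actor that wanders through space on its own in random directions.
; On Tick the authority picks a new random direction about every five seconds through a Delay.
; Every instance moves along WorldDirection as a local offset, eases its rotation toward that direction and snaps an Arrow to it.
; Unwired leftovers would spawn and possess an attached Character_SpaceShip, or pass the current transform to a location-setting custom event.
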(event `self.ReceiveBeginPlay`)

(event `self.ReceiveTick`
  (params (DeltaSeconds :type "Float (single-precision)"))
  (bind _returnvalue (`GameplayStatics.GetWorldDeltaSeconds`))
  (bind _world_direction (`self.World Direction`))
  (`|ExecutionSequence`
    (:`then_0`
      (`/Engine/EditorBlueprintResources/ActorMacros.Switch Has Authority`
        (:`Authority`
          (`KismetSystemLibrary.Delay` 5.0)
          (set `self.World Direction` (`KismetMathLibrary.RandomUnitVector`)))))
    (:`then_1`
      (`self.K2_AddActorLocalOffset` (* _world_direction _returnvalue 2000.0))
      (`self.K2_SetActorRotation` (`KismetMathLibrary.RInterpTo` (`self.K2_GetActorRotation`) (`KismetMathLibrary.Conv_VectorToRotator` _world_direction) _returnvalue 0.5))
      (`SceneComponent.K2_SetWorldRotation` (`self.Arrow`) (`KismetMathLibrary.Conv_VectorToRotator` (`self.World Direction`)) false false))))

(event `CustomEvent_0`
  (params (NewLocation :type "Vector Structure") (NewRotation :type "Rotator Structure"))
  (`self.K2_SetActorLocationAndRotation` NewLocation NewRotation))

(fn `UserConstructionScript`)