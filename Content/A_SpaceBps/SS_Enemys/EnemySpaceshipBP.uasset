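; Enemy spaceship that flies forward, takes damage and carries a widget health bar with a hit animation.
; On authority, Tick eases rotation toward TargetDirection and projects a lead point from its velocity and projectile travel time to player 0.
; That point positions a billboard and orients a distance-scaled Scene component, while sphere trace results go unused.
; Damage notifies the causer, and health below zero spawns an explosion and destroys the ship.
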(event `self.ReceiveBeginPlay`
  (`self.Setup Health Bar`))

(event `self.ReceiveTick`
  (params (DeltaSeconds :type "Float (single-precision)"))
  (bind _returnvalue (`self.K2_GetActorLocation`))
  (bind _scene (`self.Scene`))
  (bind _returnvalue_2 (/ (`self.GetDistanceTo` (`GameplayStatics.GetPlayerPawn` 0)) (`self.ProjectileSpeed`)))
  (bind _returnvalue_3 (+ _returnvalue (* (`self.GetVelocity`) _returnvalue_2)))
  (`/Engine/EditorBlueprintResources/ActorMacros.Switch Has Authority`
    (:`Authority`
      (`self.AddMovementInput` (`self.GetActorForwardVector`))
      (`self.K2_SetActorRotation` (`KismetMathLibrary.RInterpTo` (`self.K2_GetActorRotation`) (`KismetMathLibrary.Conv_VectorToRotator` (`self.TargetDirection`)) DeltaSeconds 1.0))
      (`KismetSystemLibrary.SphereTraceSingle` :`Start` _returnvalue :`End` _returnvalue_3 :`Radius` 1.0 :`TraceChannel` "TraceTypeQuery1" :`TraceColor` (struct :`R` 1.0 :`G` 1.0 :`B` 1.0 :`A` 1.0) :`TraceHitColor` (struct :`R` 1.0 :`G` 1.0 :`B` 1.0 :`A` 1.0))
      (`KismetSystemLibrary.SphereTraceSingle` :`Start` _returnvalue_3 :`End` _returnvalue_3 :`Radius` 500.0 :`TraceChannel` "TraceTypeQuery1" :`TraceColor` (struct :`R` 1.0 :`G` 1.0 :`B` 1.0 :`A` 1.0) :`TraceHitColor` (struct :`R` 1.0 :`G` 1.0 :`B` 1.0 :`A` 1.0))
      (`SceneComponent.K2_SetWorldLocation` (`self.Billboard`) _returnvalue_3 false false)
      (`SceneComponent.SetRelativeScale3D` _scene (`KismetMathLibrary.MakeVector` (* _returnvalue_2 10.0) 1.0 1.0))
      (`SceneComponent.K2_SetWorldRotation` _scene (`KismetMathLibrary.FindLookAtRotation` _returnvalue _returnvalue_3) false false))))

(event `self.ReceiveAnyDamage`
  (params (Damage :type "Float (single-precision)") (DamageType :type "DamageType Object Reference") (InstigatedBy :type "Controller Object Reference") (DamageCauser :type "Actor Object Reference"))
  (bind _output_get (set `self.Health` (- (`self.Health`) Damage)))
  (message `/Game/Characters/SpaceInterface.On Enemy Receive Hit` DamageCauser self)
  (`KismetSystemLibrary.PrintString` (`KismetStringLibrary.Conv_DoubleToString` _output_get))
  (if (< (`self.Health`) 0.0)
    (`self.Rep Destroy Emitter`)
    (`self.K2_DestroyActor`)))

(event `/Game/Characters/SpaceInterface.Play Health Bar Anim`
  (bind _as_enemy_health_bar (`self.As Enemy Health Bar`))
  (`UserWidget.PlayAnimation` _as_enemy_health_bar (`/Game/A_SpaceBps/Widgets/EnemyHealthBar.OnHit` _as_enemy_health_bar) 0.0 1 "Forward" 1.0 true))

(event `Rep Destroy Emitter`
  (`GameplayStatics.SpawnEmitterAtLocation` "/Game/Realistic_Starter_VFX_Pack_Vol2/Particles/Explosion/P_Explosion_Big_B.P_Explosion_Big_B" (`self.K2_GetActorLocation`) (struct) (10.0 10.0 10.0)))

(fn `Get Health`
  (returns (Health :type "Float (double-precision)") (`Max Health` :type "Float (double-precision)"))
  (return (`self.Health`) (`self.MaxHealth`)))

(fn `Get Space Movement Comp`
  (returns (`Space Mov Comp` :type "/Game/Characters/SpaceCharacterMovement Object Reference"))
  (return null))

(fn `Get Space Velocity`
  (returns (Velocity :type "Vector Structure"))
  (return (0.0 0.0 0.0)))

(fn `Setup Health Bar`
  (bind _asenemy_health_bar (cast `/Game/A_SpaceBps/Widgets/EnemyHealthBar` (`WidgetComponent.GetWidget` (`self.Widget`))))
  (set `self.As Enemy Health Bar` _asenemy_health_bar)
  (set `/Game/A_SpaceBps/Widgets/EnemyHealthBar.OwnerShip` self _asenemy_health_bar))

(fn `TargetGetVelocity`
  (params (Target :type "Actor Object Reference"))
  (returns (ReturnValue :type "Vector Structure"))
  (bind _ascharacter_space_ship (cast `/Game/A_SpaceBps/Characters/Character_SpaceShip` Target)
    (:`then`
      (bind _velocity (message `/Game/Characters/SpaceInterface.Get Space Velocity` _ascharacter_space_ship))
      (return _velocity))
    (:`CastFailed`
      (return (`self.GetVelocity` Target)))))

(fn `UserConstructionScript`)