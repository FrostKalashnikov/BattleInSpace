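; Master player character for a multiplayer space game, handling input, weapons, interaction and HUD creation.
; Feeds movement, look, sprint, jump and mode toggling into SpaceCharacterMovement, whose rotation also takes timer-decayed recoil.
; Switches between two child-actor weapons using an OnRep visibility flag, forwarding fire, reload and timeline-driven spring-arm ADS.
; Montages play locally then relay via server to multicast, while interaction sends overlapping component tags through SpaceInterface.
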(event `InputAction|Jump`
  (params (Key :type "Key Structure"))
  (:`Pressed`
    (`/Game/Characters/SpaceCharacterMovement.Jump Event` (`self.SpaceCharacterMovement`))))

(event `self.ReceiveTick`
  (params (DeltaSeconds :type "Float (single-precision)"))
  (if (`self.IsLocallyControlled`)
    (`/Game/Characters/SpaceCharacterMovement.Mouse Turn / Look` (`self.SpaceCharacterMovement`) (`self.GetInputAxisValue`) (`self.GetInputAxisValue`))
    (`/Game/Characters/SpaceCharacterMovement.Movement Input ` (`self.SpaceCharacterMovement`) (`self.GetInputAxisValue`) (`self.GetInputAxisValue`) (`self.GetInputAxisValue`))))

(event `Key|LeftShift`
  (params (Key :type "Key Structure"))
  (bind _spacecharactermovement (`self.SpaceCharacterMovement`))
  (:`Pressed`
    (set `/Game/Characters/SpaceCharacterMovement.Movement Speed` 600.0 _spacecharactermovement)
    (set `/Game/Characters/SpaceCharacterMovement.IsRunning` true _spacecharactermovement))
  (:`Released`
    (set `/Game/Characters/SpaceCharacterMovement.Movement Speed` 300.0 _spacecharactermovement)
    (set `/Game/Characters/SpaceCharacterMovement.IsRunning` false _spacecharactermovement)))

(event `self.ReceiveBeginPlay`
  (bind _childactor (`ChildActorComponent.ChildActor` (`self.Weapon_2`)))
  (`|ExecutionSequence`
    (:`then_0`
      (`/Engine/EditorBlueprintResources/ActorMacros.Switch Has Authority`
        (:`Authority`
          (`self.SetOwner` _childactor self)
          (`self.SetOwner` (`ChildActorComponent.ChildActor` (`self.Weapon_1`)) self)
          (`|ExecutionSequence`
            (:`then_0`
              (bind _asmaster_weapon_bp (cast `/Game/A_SpaceBps/Weapons/MasterWeaponBp` _childactor))
              (set `/Game/A_SpaceBps/Weapons/MasterWeaponBp.OwnerCharacter` self _asmaster_weapon_bp))
            (:`then_1`
              (bind _asmaster_weapon_bp_2 (cast `/Game/A_SpaceBps/Weapons/MasterWeaponBp` (`ChildActorComponent.ChildActor` (`self.Weapon_1`))))
              (set `/Game/A_SpaceBps/Weapons/MasterWeaponBp.OwnerCharacter` self _asmaster_weapon_bp_2))))))
    (:`then_1`
      (if (`self.IsLocallyControlled`)
        (bind _returnvalue (`|CreateWidget` "/Game/A_SpaceBps/Widgets/MasterInterface.MasterInterface_C"))
        (set `self.MasterInterfaceUI` _returnvalue)
        (`UserWidget.AddToViewport` _returnvalue 0)))))

(event `Key|LeftMouseButton`
  (params (Key :type "Key Structure"))
  (bind _asmaster_weapon_bp (`self.Get Weapon`))
  (bind _returnvalue (and (`self.Can Fire`) (not (`self.IsSwitching`))))
  (:`Pressed`
    (if _returnvalue
      (`/Game/A_SpaceBps/Weapons/MasterWeaponBp.Start Fire` _asmaster_weapon_bp)))
  (:`Released`
    (if _returnvalue
      (`/Game/A_SpaceBps/Weapons/MasterWeaponBp.End Fire` _asmaster_weapon_bp))))

(event `Key|One`
  (params (Key :type "Key Structure"))
  (bind (_asmaster_weapon_bp _weapondata) (`self.Get Weapon`))
  (bind _asmaster_weapon_bp_2 (`self.Get Weapon`))
  (:`Pressed`
    (`SceneComponent.SetHiddenInGame` (`self.Weapon_1`) false false)
    (`SceneComponent.SetHiddenInGame` (`self.Weapon_2`) true false)
    (`|ExecutionSequence`
      (:`then_0`
        (`/Game/A_SpaceBps/Weapons/MasterWeaponBp.End Fire` _asmaster_weapon_bp_2 :!label _label)
        (`KismetSystemLibrary.K2_ClearTimer` _asmaster_weapon_bp_2 "FinishReload")
        (set `/Game/A_SpaceBps/Weapons/MasterWeaponBp.Is Reloading` false _asmaster_weapon_bp_2)
        (`self.Reverse ADS`)
        (if (`.CanADS_61_9B90487444CA273BED191C99BA450DFC` (break `/Game/A_SpaceBps/Weapons/WeaponData_S` _weapondata))
          (`/Game/A_SpaceBps/Weapons/MasterWeaponBp.Set ADS Status` _asmaster_weapon_bp false)))
      (:`then_1`
        (`self.Set Is Primary` true)
        (`self.Play Montage Event` null (`.EquipMontage_35_E45C5C7048786D53ED1984AF887A3DA7` (break `/Game/A_SpaceBps/Weapons/WeaponData_S` (`/Game/A_SpaceBps/Weapons/MasterWeaponBp.WeaponData` (`self.Get Weapon`)))) :!label _label_2)
        (set `self.IsSwitching` true)
        (`KismetSystemLibrary.RetriggerableDelay` 0.5)
        (set `self.IsSwitching` false)))))

(event `Key|Two`
  (params (Key :type "Key Structure"))
  (:`Pressed`
    (`SceneComponent.SetHiddenInGame` (`self.Weapon_2`) false false)
    (`SceneComponent.SetHiddenInGame` (`self.Weapon_1`) true false)
    (`|ExecutionSequence`
      (:`then_0`
        (goto _label))
      (:`then_1`
        (`self.Set Is Primary` false)
        (goto _label_2)))))

(event `Key|RightMouseButton`
  (params (Key :type "Key Structure"))
  (bind (_asmaster_weapon_bp _weapondata) (`self.Get Weapon`))
  (bind ((`CanADS_61_9B90487444CA273BED191C99BA450DFC` _canads)) (break `/Game/A_SpaceBps/Weapons/WeaponData_S` _weapondata))
  (:`Pressed`
    (if _canads
      (`self.Play ADS`)
      (`/Game/A_SpaceBps/Weapons/MasterWeaponBp.Set ADS Status` _asmaster_weapon_bp true)))
  (:`Released`
    (if _canads
      (`self.Reverse ADS`)
      (`/Game/A_SpaceBps/Weapons/MasterWeaponBp.Set ADS Status` _asmaster_weapon_bp false))))

(event `Key|E`
  (params (Key :type "Key Structure"))
  (:`Pressed`
    (`self.Interact Event`)))

(event `Key|R`
  (params (Key :type "Key Structure"))
  (:`Pressed`
    (if (not (`self.IsSwitching`))
      (`/Game/A_SpaceBps/Weapons/MasterWeaponBp.Reload Weapon` (`self.Get Weapon`)))))

(event `Key|T`
  (params (Key :type "Key Structure"))
  (bind _spacecharactermovement (`self.SpaceCharacterMovement`))
  (:`Pressed`
    (`/Engine/EditorBlueprintResources/StandardMacros.FlipFlop`
      (:`A`
        (set `/Game/Characters/SpaceCharacterMovement.Movement Mode` "NewEnumerator4" _spacecharactermovement))
      (:`B`
        (set `/Game/Characters/SpaceCharacterMovement.Movement Mode` "NewEnumerator1" _spacecharactermovement)))))

(event `Play ADS`
  (bind _springarm (`self.SpringArm`))
  (bind (_direction _socket_offset _arm_length) (`Timeline|ADS` :!label _label_3)
    (:`Update`
      (set `SpringArmComponent.SocketOffset` _socket_offset _springarm)
      (set `SpringArmComponent.TargetArmLength` _arm_length _springarm))))

(event `Reverse ADS`
  (goto _label_3 :!via `Reverse`))

(event `Attach To Component On Multi`
  (params (`Actor Target` :type "Actor Object Reference") (Parent :type "SceneComponent Object Reference"))
  (`self.K2_AttachToComponent` `Actor Target` Parent "None" "SnapToTarget" "SnapToTarget" "SnapToTarget" true))

(event `Detach From Actor On Multi`
  (params (`Actor To Detach` :type "Actor Object Reference"))
  (`self.K2_DetachFromActor` `Actor To Detach` "KeepWorld" "KeepWorld" "KeepWorld"))

(event `Play Montage On Server`
  (params (Character :type "Character Object Reference") (AnimMontage :type "AnimMontage Object Reference") (InPlayRate :type "Float (single-precision)" :default 1.0) (StartSectionName :type Name))
  (`self.Play Montage On Multi` Character AnimMontage InPlayRate StartSectionName))

(event `Play Montage On Multi`
  (params (Character :type "Character Object Reference") (AnimMontage :type "AnimMontage Object Reference") (InPlayRate :type "Float (single-precision)" :default 1.0) (StartSectionName :type Name))
  (if (not (`self.IsLocallyControlled`))
    (`self.PlayAnimMontage` AnimMontage InPlayRate StartSectionName)))

(event `Play Montage Event`
  (params (Character :type "Character Object Reference") (AnimMontage :type "AnimMontage Object Reference") (InPlayRate :type "Float (single-precision)" :default 1.0) (StartSectionName :type Name))
  (`self.PlayAnimMontage` AnimMontage InPlayRate StartSectionName)
  (`self.Play Montage On Server` Character AnimMontage InPlayRate StartSectionName))

(event `Interact by Comp On Server`
  (params (Target :type "Object Object Reference") (InteractionTag :type Name) (Character :type "Character Object Reference") (Controller :type "PlayerController Object Reference"))
  (message `/Game/Characters/SpaceInterface.Interact by CompTag` Target InteractionTag Character Controller))

(event `Set Is Primary`
  (params (`IsPrimaryWeapon?` :type Boolean))
  (set `self.IsPrimaryWeapon?` `IsPrimaryWeapon?`))

(event `Play Montage Everyone Event`
  (params (Selection :type String))
  (`self.Play Fire Montage On Server` Selection)
  (message `/Game/Characters/SpaceInterface.Play Montage Everyone` (`SkeletalMeshComponent.GetAnimInstance` (`self.Mesh`)) Selection))

(event `Play Fire Montage On Server`
  (params (Selection :type String))
  (`self.Play Fire Montage On Multi` Selection))

(event `Play Fire Montage On Multi`
  (params (Selection :type String))
  (if (not (`self.IsLocallyControlled`))
    (message `/Game/Characters/SpaceInterface.Play Montage Everyone` (`SkeletalMeshComponent.GetAnimInstance` (`self.Mesh`)) Selection)))

(fn `Add Recoil`
  (params (Recoil :type "Vector2D Structure"))
  (bind (_recoil_x _recoil_y) (`KismetMathLibrary.BreakVector2D` (`local.Recoil`)))
  (bind (_rotation_x _rotation_y) (`KismetMathLibrary.BreakVector2D` (`/Game/Characters/SpaceCharacterMovement.Rotation` (`self.SpaceCharacterMovement`))))
  (set `self.RecoilAmount` (+ Recoil (`self.RecoilAmount`)))
  (set `/Game/Characters/SpaceCharacterMovement.Rotation` (`KismetMathLibrary.MakeVector2D` (+ _rotation_x _recoil_x) (+ _rotation_y _recoil_y)) (`self.SpaceCharacterMovement`))
  (`KismetSystemLibrary.K2_SetTimer` null "ResetingRecoil" 0.01 true))

(fn `Get Weapon`
  (returns (`AsMaster Weapon Bp` :type "/Game/A_SpaceBps/Weapons/MasterWeaponBp Object Reference") (WeaponData :type "/Game/A_SpaceBps/Weapons/WeaponData_S Structure"))
  (bind _asmaster_weapon_bp (cast `/Game/A_SpaceBps/Weapons/MasterWeaponBp` (`ChildActorComponent.ChildActor` (select `bool` (`self.IsPrimaryWeapon?`) :`false` (`self.Weapon_2`) :`true` (`self.Weapon_1`)))))
  (return _asmaster_weapon_bp (`/Game/A_SpaceBps/Weapons/MasterWeaponBp.WeaponData` _asmaster_weapon_bp)))

(fn `Interact Event`
  (for _array_element (`self.GetOverlappingComponents`)
    (bind _output (`|GetArrayItem` (`ActorComponent.ComponentTags` _array_element)))
    (`KismetSystemLibrary.PrintString` (`KismetStringLibrary.Conv_NameToString` _output))
    (bind _returnvalue (`ActorComponent.GetOwner` _array_element))
    (if (and (!= _output "None") (`KismetSystemLibrary.DoesImplementInterface` _returnvalue "/Game/Characters/SpaceInterface.SpaceInterface_C"))
      (`self.Interact by Comp On Server` _returnvalue _output self (`GameplayStatics.GetPlayerController` 0))
      (break))))

(fn `OnRep_IsPrimaryWeapon?`
  (bind _weapon_1 (`self.Weapon_1`))
  (bind _weapon_2 (`self.Weapon_2`))
  (if (`self.IsPrimaryWeapon?`)
    (`SceneComponent.SetHiddenInGame` _weapon_1 false false)
    (`SceneComponent.SetHiddenInGame` _weapon_2 true false)
    (else
      (`SceneComponent.SetHiddenInGame` _weapon_2 false false)
      (`SceneComponent.SetHiddenInGame` _weapon_1 true false))))

(fn `ResetingRecoil`
  (locals (RecoilToRemove :type "Vector2D Structure"))
  (bind _spacecharactermovement (`self.SpaceCharacterMovement`))
  (set `local.RecoilToRemove` (`KismetMathLibrary.Vector2DInterpTo` (`self.RecoilAmount`) (0.0 0.0) 0.01 2.0))
  (set `/Game/Characters/SpaceCharacterMovement.Rotation` (- (`/Game/Characters/SpaceCharacterMovement.Rotation` _spacecharactermovement) (- (`self.RecoilAmount`) (`local.RecoilToRemove`))) _spacecharactermovement)
  (set `self.RecoilAmount` (`local.RecoilToRemove`))
  (if (== (`self.RecoilAmount`) (0.0 0.0))
    (`KismetSystemLibrary.K2_ClearTimer` null "Reseting Recoil")))

(fn `UserConstructionScript`
  (set `/Game/Characters/SpaceCharacterMovement.SpringArmRef` (`self.SpringArm`) (`self.SpaceCharacterMovement`)))