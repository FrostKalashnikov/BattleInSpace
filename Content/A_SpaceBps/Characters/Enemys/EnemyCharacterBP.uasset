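; Enemy character base with custom server-side wandering movement that faces its Target when one is valid, otherwise its travel direction.
; On the server, Tick eases Velocity toward a random direction and moves by swept offsets, re-rolling the direction when a sphere trace is blocked or after a delay.
; A downward sphere trace holds capsule height above ground or applies gravity.
; Remote instances smoothly interpolate mesh yaw toward MeshRotation.
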(event `self.ReceiveBeginPlay`
  (`/Engine/EditorBlueprintResources/ActorMacros.Switch Has Authority`
    (:`Authority`
      (set `self.DirectionVec` (`KismetMathLibrary.MakeVector` (`KismetMathLibrary.Conv_IntToDouble` (`KismetMathLibrary.RandomIntegerInRange` -1 1)) (`KismetMathLibrary.Conv_IntToDouble` (`KismetMathLibrary.RandomIntegerInRange` -1 1)))))))

(event `self.ReceiveTick`
  (params (DeltaSeconds :type "Float (single-precision)"))
  (bind _velocityarrow (`self.VelocityArrow`))
  (bind _returnvalue (`SceneComponent.K2_GetComponentLocation` _velocityarrow))
  (`/Engine/EditorBlueprintResources/ActorMacros.Switch Has Authority`
    (:`Authority`
      (`self.Update Velocity`)
      (`self.Update Direction`)
      (`self.Update Height`)
      (`|ExecutionSequence`
        (:`then_0`
          (bind (_outhit _returnvalue_2) (`KismetSystemLibrary.SphereTraceSingle` :`Start` _returnvalue :`End` (+ _returnvalue (* (`SceneComponent.GetForwardVector` _velocityarrow) (`KismetMathLibrary.SelectFloat` 0.0 100.0 (== (`KismetMathLibrary.VSize` (`self.DirectionVec`)) 0.0)))) :`Radius` (`CapsuleComponent.CapsuleRadius` (`self.CapsuleComponent`)) :`TraceChannel` "TraceTypeQuery1" :`DrawDebugType` (`self.Draw Debug Type`)))
          (if (not _returnvalue_2)
            (`KismetSystemLibrary.Delay` 10.0))
          (bind _output_get (set `self.DirectionVec` (`KismetMathLibrary.Normal` (`KismetMathLibrary.MakeVector` (`KismetMathLibrary.RandomFloatInRange` -1.0 1.0) (`KismetMathLibrary.RandomFloatInRange` -1.0 1.0))) :!label _label))
          (if (== _output_get (0.0 0.0 0.0))
            (`KismetSystemLibrary.Delay` 1.0)
            (goto _label)))
        (:`then_1`
          (`self.K2_AddActorLocalOffset` (* (`self.Velocity`) (`self.Movement Speed`) (`GameplayStatics.GetWorldDeltaSeconds`)) true))))
    (:`Remote`
      (bind _output_get_2 (set `self.Relative Rotation` (`KismetMathLibrary.RInterpTo` (`self.Relative Rotation`) (`self.Mesh Rotation`) (`GameplayStatics.GetWorldDeltaSeconds`) 7.0)))
      (`SceneComponent.K2_SetRelativeRotation` (`self.Mesh`) (`KismetMathLibrary.MakeRotator` 0.0 0.0 (.yaw _output_get_2)) false false))))

(event `Set Mesh Rotation On Multi`
  (params (NewRotation :type "Rotator Structure"))
  (`SceneComponent.K2_SetRelativeRotation` (`self.Mesh`) NewRotation false false))

(fn `DirectionOnPath`
  (bind _velocity (`self.Velocity`))
  (bind _returnvalue (`KismetMathLibrary.Conv_VectorToRotator` _velocity))
  (if (!= _velocity (0.0 0.0 0.0))
    (set `self.Mesh Rotation` (`KismetMathLibrary.ComposeRotators` _returnvalue (`KismetMathLibrary.MakeRotator` 0.0 0.0 -90.0)))
    (`SceneComponent.K2_SetRelativeRotation` (`self.LookArrow`) (`KismetMathLibrary.MakeRotator` 0.0 0.0 (.yaw _returnvalue)) false false)))

(fn `DirectionOnTarget`
  (`SceneComponent.K2_SetWorldRotation` (`self.LookArrow`) (`KismetMathLibrary.FindLookAtRotation` (`self.K2_GetActorLocation`) (`self.K2_GetActorLocation` (`self.Target`))) false false)
  (set `self.Mesh Rotation` (`KismetMathLibrary.ComposeRotators` (`SceneComponent.RelativeRotation` (`self.LookArrow`)) (`KismetMathLibrary.MakeRotator` 0.0 0.0 -90.0))))

(fn `Update Direction`
  (bind (_returnvalue_roll _returnvalue_pitch _returnvalue_yaw) (`KismetMathLibrary.BreakRotator` (`KismetMathLibrary.NormalizedDeltaRotator` (`KismetMathLibrary.Conv_VectorToRotator` (`self.Velocity`)) (`KismetMathLibrary.ComposeRotators` (`SceneComponent.RelativeRotation` (`self.Mesh`)) (struct :`Yaw` 90.0)))))
  (set `self.Direction` _returnvalue_yaw)
  (`self.Target`
    (:`then`
      (`self.DirectionOnTarget`))
    (:`else`
      (`self.DirectionOnPath`))))

(fn `Update Height`
  (bind _returnvalue (`self.K2_GetActorLocation`))
  (bind _capsulecomponent (`self.CapsuleComponent`))
  (bind _returnvalue_2 (- (+ (`CapsuleComponent.CapsuleHalfHeight` _capsulecomponent) 10.0) (`CapsuleComponent.CapsuleRadius` _capsulecomponent)))
  (bind _returnvalue_3 (- _returnvalue_2 5.0))
  (bind (_outhit _returnvalue_4) (`KismetSystemLibrary.SphereTraceSingleForObjects` :`Start` _returnvalue :`End` (+ _returnvalue (* (`self.GetActorUpVector`) (* _returnvalue_2 -1.0))) :`Radius` (`CapsuleComponent.CapsuleRadius` _capsulecomponent) :`ObjectTypes` (`|MakeArray` "ObjectTypeQuery1" "ObjectTypeQuery2" :!type "EObjectTypeQuery Enum") :`bTraceComplex` true :`DrawDebugType` (`self.Draw Debug Type`)))
  (if _returnvalue_4
    (bind (_bblockinghit _binitialoverlap _time _distance) (`GameplayStatics.BreakHitResult` _outhit))
    (if (`KismetMathLibrary.NearlyEqual_FloatFloat` _distance _returnvalue_3 1.0)
      _
      (elif (< _distance _returnvalue_3)
        (`self.K2_AddActorLocalOffset` (`KismetMathLibrary.MakeVector` 0.0 0.0 (- _returnvalue_3 _distance)))
        (elif (> _distance _returnvalue_3)
          (`self.K2_AddActorLocalOffset` (`KismetMathLibrary.MakeVector` 0.0 0.0 (- _returnvalue_3 _distance))))))
    (else
      (`self.K2_AddActorLocalOffset` (`KismetMathLibrary.MakeVector` 0.0 0.0 (* (`GameplayStatics.GetWorldDeltaSeconds`) (`self.GravityForce`))) true))))

(fn `Update Velocity`
  (bind _output_get (set `self.Velocity` (`KismetMathLibrary.VInterpTo` (`self.Velocity`) (`self.DirectionVec`) (`GameplayStatics.GetWorldDeltaSeconds`) (`self.Velocity Interp Speed`))))
  (`SceneComponent.K2_SetRelativeRotation` (`self.VelocityArrow`) (`KismetMathLibrary.Conv_VectorToRotator` _output_get) false false))

(fn `UserConstructionScript`)