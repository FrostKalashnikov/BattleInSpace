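; SS_MasterWeaponBP is a controllable weapon with mouse look and automatic projectile fire.
; Mouse axes drive controller pitch and yaw, while holding left mouse opens a Gate that loops through a short Delay to repeat shots until release.
; Each shot spawns ProjectileMasterBP at FireOut, rotated toward a distant point along the camera's forward vector, with assault rifle tracer and metal impact effects.
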(event `InputAxis|Look Up / Down Mouse`
  (params (AxisValue :type "Float (single-precision)"))
  (`self.AddControllerPitchInput` AxisValue))

(event `InputAxis|Turn Right / Left Mouse`
  (params (AxisValue :type "Float (single-precision)"))
  (`self.AddControllerYawInput` AxisValue))

(event `Key|LeftMouseButton`
  (params (Key :type "Key Structure"))
  (bind _camera (`self.Camera`))
  (bind _returnvalue (`SceneComponent.K2_GetComponentLocation` (`self.FireOut`)))
  (:`Pressed`
    (`|ExecutionSequence`
      (:`then_0`
        (goto _label :!via `Open`))
      (:`then_1`
        (`/Engine/EditorBlueprintResources/StandardMacros.Gate` true :!label _label
          (:`Exit`
            (`|SpawnActorFromClass` "/Game/A_SpaceBps/Projectile/ProjectileMasterBP.ProjectileMasterBP_C" (`KismetMathLibrary.MakeTransform` _returnvalue (`KismetMathLibrary.FindLookAtRotation` _returnvalue (+ (`SceneComponent.K2_GetComponentLocation` _camera) (* (`SceneComponent.GetForwardVector` _camera) 10000.0)))) "AlwaysSpawn" "OverrideRootScale" null null "/Game/SciFiWeapLight/FX/Particles/P_AssaultRifle_Tracer_Light.P_AssaultRifle_Tracer_Light" "/Game/SciFiWeapLight/FX/Particles/P_Impact_Metal_Medium_Light.P_Impact_Metal_Medium_Light" 15.0 (struct :`G` 1.0 :`B` 0.113013 :`A` 1.0) false (`self.Instigator_0`))
            (`KismetSystemLibrary.Delay` 0.2)
            (goto _label))))))
  (:`Released`
    (goto _label :!via `Close`)))

(fn `UserConstructionScript`)