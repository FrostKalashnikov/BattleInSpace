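; Master weapon Blueprint whose mesh, effects, ammo, damage and handling come from a WeaponData struct.
; Timers drive single or automatic fire, cooldown and reload, while montages and recoil go through OwnerCharacter.
; Shots trace from the camera to aim a spread-randomized projectile from the muzzle, spawned through a server event.
; Fire FX play locally and reach non-owners via server-to-multicast events; aim-down-sights toggles the struct's TypeID.
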(event `Set ADS Status`
  (params (Condition :type Boolean))
  (bind _weapondata (`self.WeaponData`))
  (`self.Set ADS Status On Server` Condition)
  (if Condition
    (setmembers `/Game/A_SpaceBps/Weapons/WeaponData_S` :`StructRef` _weapondata :`TypeID` 1 :!label _label)
    (else
      (setmembers `/Game/A_SpaceBps/Weapons/WeaponData_S` :`StructRef` _weapondata :`TypeID` 0 :!label _label_2))))

(event `Play FX/Sound On Server`
  (`self.Play FX/Sound On Multi`))

(event `Set ADS Status On Server`
  (params (Condition :type Boolean))
  (if Condition
    (goto _label)
    (else
      (goto _label_2))))

(event `Play FX/Sound On Multi`
  (bind _audio (`self.Audio`))
  (`self.Is Not Owner`
    (:`Is Not`
      (`AudioComponent.SetSound` _audio (`.FireSound_19_301721BC4674876C43358AA9D4C4BFF5` (break `/Game/A_SpaceBps/Weapons/WeaponData_S` (`self.WeaponData`))))
      (`AudioComponent.Play` _audio 0.0)
      (`ActorComponent.SetActive` (`self.MuzzleFX`) true true))))

(event `Spawn Projectile On Server`
  (params (SpawnTransform :type "Transform Structure") (SpaceshipRef :type "/Game/Spaceship/SpaceShip_Blueprint Object Reference") (Instigator :type "Pawn Object Reference"))
  (bind ((`Damage_55_1C63A6174F7749C6A3AF389571E40BF7` _damage) (`ImpactFX_27_B80CD133435A8C273B876A9C2700F745` _impactfx) (`TraceFX_39_BE9825FC4D038A883243C1B85A27F363` _tracefx)) (break `/Game/A_SpaceBps/Weapons/WeaponData_S` (`self.WeaponData`)))
  (`|SpawnActorFromClass` "/Game/A_SpaceBps/Projectile/ProjectileMasterBP.ProjectileMasterBP_C" SpawnTransform "AlwaysSpawn" "OverrideRootScale" Instigator SpaceshipRef _tracefx _impactfx _damage 50000.0 (struct :`R` 0.05 :`G` 0.176667 :`B` 1.0 :`A` 1.0) false Instigator))

(event `Reload Weapon`
  (bind ((`CanADS_61_9B90487444CA273BED191C99BA450DFC` _canads) (`CurrentAmmo_10_A1AC807948BA9E9808B6E58FDA0DB6B9` _currentammo) (`MaxAmmo_9_9F5F815346EDE0F32E81938D31E14DD5` _maxammo) (`ReloadDuration_59_133A485E48DC7E8E52B6B0BA046BF029` _reloadduration)) (break `/Game/A_SpaceBps/Weapons/WeaponData_S` (`self.WeaponData`)))
  (if (and (!= _currentammo _maxammo) (not (`self.Is Reloading`)))
    (`KismetSystemLibrary.K2_SetTimer` null "FinishReload" _reloadduration)
    (`/Game/Characters/MasterCharacterBP.Play Montage Everyone Event` (`self.OwnerCharacter`) "Reload")
    (set `self.Is Reloading` true)))

(fn `End Fire`
  (`KismetSystemLibrary.K2_ClearTimer` null "FireEvent"))

(fn `FinishReload`
  (bind _weapondata (`self.WeaponData`))
  (setmembers `/Game/A_SpaceBps/Weapons/WeaponData_S` :`StructRef` _weapondata :`CurrentAmmo` (`.MaxAmmo_9_9F5F815346EDE0F32E81938D31E14DD5` (break `/Game/A_SpaceBps/Weapons/WeaponData_S` _weapondata)))
  (set `self.Is Reloading` false))

(fn `FireEvent`
  (bind _returnvalue (`GameplayStatics.GetPlayerCameraManager` 0))
  (bind _audio (`self.Audio`))
  (bind _weapondata (`self.WeaponData`))
  (bind ((`Spread_49_95AFF9BB433317EDB361D393CCBB3A33` _spread) (`RecoilScale_51_205AC327494F475B331F519DFC9167F7` _recoilscale) (`CurrentAmmo_10_A1AC807948BA9E9808B6E58FDA0DB6B9` _currentammo)) (break `/Game/A_SpaceBps/Weapons/WeaponData_S` (`self.WeaponData`)))
  (bind ((`FireRate_13_E794F36840A57B2513877FB60238A7AC` _firerate) (`FireSound_19_301721BC4674876C43358AA9D4C4BFF5` _firesound)) (break `/Game/A_SpaceBps/Weapons/WeaponData_S` _weapondata))
  (bind _returnvalue_2 (`PlayerCameraManager.GetCameraLocation` _returnvalue))
  (bind _returnvalue_3 (`SceneComponent.GetSocketLocation` (`self.Mesh`) "Muzzle"))
  (bind _returnvalue_4 (`KismetMathLibrary.RandomFloatInRange` (* _spread -1.0) _spread))
  (if (and (> (`.CurrentAmmo_10_A1AC807948BA9E9808B6E58FDA0DB6B9` (break `/Game/A_SpaceBps/Weapons/WeaponData_S` _weapondata)) 0) (not (`self.Is Reloading`)) (not (`self.InColdown`)))
    (set `self.InColdown` true)
    (`KismetSystemLibrary.K2_SetTimer` null "ResetFireColdown" (* _firerate 0.8))
    (`ActorComponent.SetActive` (`self.MuzzleFX`) true true)
    (`AudioComponent.SetSound` _audio _firesound)
    (`AudioComponent.Play` _audio 0.0)
    (`self.Play FX/Sound On Server`)
    (`KismetSystemLibrary.K2_ClearTimer` null "FinishReload")
    (`/Game/Characters/MasterCharacterBP.Play Montage Everyone Event` (`self.OwnerCharacter`) "Fire")
    (bind (_outhit _returnvalue_5) (`KismetSystemLibrary.LineTraceSingle` _returnvalue_2 (+ _returnvalue_2 (* (`self.GetActorForwardVector` _returnvalue) 10000.0)) "TraceTypeQuery1"))
    (setmembers `/Game/A_SpaceBps/Weapons/WeaponData_S` :`StructRef` (`self.WeaponData`) :`CurrentAmmo` (- _currentammo 1))
    (bind (_bblockinghit _binitialoverlap _time _distance _location _impactpoint _normal _impactnormal _physmat _hitactor _hitcomponent _hitbonename _bonename _hititem _elementindex _faceindex _tracestart _traceend) (`GameplayStatics.BreakHitResult` _outhit))
    (`self.Spawn Projectile On Server` (`KismetMathLibrary.MakeTransform` _returnvalue_3 (`KismetMathLibrary.ComposeRotators` (`KismetMathLibrary.FindLookAtRotation` _returnvalue_3 (`KismetMathLibrary.SelectVector` _impactpoint _traceend _returnvalue_5)) (`KismetMathLibrary.MakeRotator` 0.0 (`KismetMathLibrary.RandomFloatInRange` (* _spread -1.0) _spread) _returnvalue_4))) (`/Game/Characters/MasterCharacterBP.SpaceShipRef` (`self.OwnerCharacter`)) (`GameplayStatics.GetPlayerPawn` 0))
    (bind _ownercharacter (`self.OwnerCharacter`)
      (:`then`
        (`/Game/Characters/MasterCharacterBP.Add Recoil` _ownercharacter (`KismetMathLibrary.MakeVector2D` _returnvalue_4 _recoilscale)))
      (:`else`))))

(fn `ResetFireColdown`
  (set `self.InColdown` false))

(fn `Start Fire`
  (bind ((`CanADS_61_9B90487444CA273BED191C99BA450DFC` _canads) (`FireRate_13_E794F36840A57B2513877FB60238A7AC` _firerate) (`FireTypeAuto_46_491B85834490424CA25E3E9BD975D399` _firetypeauto)) (break `/Game/A_SpaceBps/Weapons/WeaponData_S` (`self.WeaponData`)))
  (`self.FireEvent`)
  (if _firetypeauto
    (`KismetSystemLibrary.K2_SetTimer` null "FireEvent" _firerate true)))

(fn `UserConstructionScript`
  (bind _mesh (`self.Mesh`))
  (bind ((`CanADS_61_9B90487444CA273BED191C99BA450DFC` _canads) (`Spread_49_95AFF9BB433317EDB361D393CCBB3A33` _spread) (`RecoilScale_51_205AC327494F475B331F519DFC9167F7` _recoilscale) (`ReloadDuration_59_133A485E48DC7E8E52B6B0BA046BF029` _reloadduration) (`Damage_55_1C63A6174F7749C6A3AF389571E40BF7` _damage) (`Mesh_16_D2ABF91E4051CF2CA45C0BBDCDAB9EF1` _mesh_2) (`SkinMaterial_43_5DB461BE40785B6B21B163B760E7CA94` _skinmaterial) (`FireMuzzleFX_22_A750344249520B4C4B535CA9C977410C` _firemuzzlefx)) (break `/Game/A_SpaceBps/Weapons/WeaponData_S` (`self.WeaponData`)))
  (`|ExecutionSequence`
    (:`then_0`
      (`SkinnedMeshComponent.SetSkinnedAssetAndUpdate` _mesh _mesh_2 true)
      (if (!= _skinmaterial null)
        (`PrimitiveComponent.SetMaterial` _mesh 0 _skinmaterial)))
    (:`then_1`
      (`ParticleSystemComponent.SetTemplate` (`self.MuzzleFX`) _firemuzzlefx))))